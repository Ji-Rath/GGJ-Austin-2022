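; BP_GoldKey is a gold key pickup that triggers end-of-level changes when the player interacts with it.
; Its Pickupable interact event deactivates and destroys the PortalKiller actor, then makes BoxEndGame visible with BlockAll collision.
; A pickup sound plays at the key's location; the key itself is not hidden or destroyed in this graph.
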(event `self.Pickupable.OnInteract`
  (params (Interactor :type "Actor Object Reference"))
  (bind _portalkiller (`self.PortalKiller`))
  (bind _boxendgame (`self.BoxEndGame`))
  (`Portal.SetActive` _portalkiller false)
  (`self.K2_DestroyActor` _portalkiller)
  (`PrimitiveComponent.SetCollisionProfileName` (`/Game/Blueprints/BP_StrangeBoxEnd.StaticMeshComponent1` _boxendgame) "BlockAll" true)
  (`self.SetActorHiddenInGame` _boxendgame false)
  (`GameplayStatics.PlaySoundAtLocation` "/Game/Assets/SoundCues/Cue_Pickup.Cue_Pickup" (`self.K2_GetActorLocation`) (struct) 1.0 1.0 0.0 null null null))

(fn `UserConstructionScript`
  (`parent.UserConstructionScript`))