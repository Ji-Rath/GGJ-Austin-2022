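; Trigger actor that locks a referenced door behind a golden key requirement, apparently at the start of the game.
; The first overlap by any actor fires its own Interactable component through a DoOnce, so overlaps alone trigger it only once.
; The interact handler switches the door's ToggleInteractable state off, adds the golden key to its usable component's needed items, and marks it locked.
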(event `self.Interactable.OnInteract`
  (params (Interactor :type "Actor Object Reference"))
  (bind _doorref (`self.DoorRef`))
  (`ToggleInteractableComponent.SetState` (`/Game/Blueprints/BP_Door.ToggleInteractable` _doorref) null false)
  (`KismetArrayLibrary.Array_AddUnique` (`/Game/Blueprints/Components/BP_ItemUsableComponent.ItemsNeeded` (`self.GetComponentByClass` _doorref "/Game/Blueprints/Components/BP_ItemUsableComponent.BP_ItemUsableComponent_C")) "/Game/Blueprints/Items/ItemData/Item_GoldenKey.Item_GoldenKey")
  (set `/Game/Blueprints/BP_Door.bLocked` true _doorref))

(event `self.ReceiveActorBeginOverlap`
  (params (OtherActor :type "Actor Object Reference"))
  (`/Engine/EditorBlueprintResources/StandardMacros.DoOnce` false
    (:`Completed`
      (`InteractableComponent.OnInteract` (`self.Interactable`) null))))

(event `self.ReceiveActorEndOverlap`
  (params (OtherActor :type "Actor Object Reference")))

(fn `UserConstructionScript`)