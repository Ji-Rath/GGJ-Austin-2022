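; Player component that lets its owner use inventory items on interactable actors.
; On BeginPlay it binds to the owner's PlayerInteractComponent interact event, then looks for a BP_ItemUsableComponent on the interacted actor.
; Each needed item found in the owner's InventoryComponent has one unit removed, firing use events on both this component and the target's.
; Items are consumed individually, without requiring the full set.
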(event `self.ReceiveBeginPlay`
  (add `PlayerInteractComponent.OnInteract` (`Actor.GetComponentByClass` (`self.GetOwner`) "/Script/InteractionSystem.PlayerInteractComponent") (delegate `Try Use Item`)))

(event `Try Use Item`
  (params (Interactable :type "InteractableComponent Object Reference"))
  (bind _returnvalue (`self.GetOwner` Interactable))
  (bind _returnvalue_2 (`self.GetOwner`))
  (bind _returnvalue_3 (`Actor.GetComponentByClass` _returnvalue "/Game/Blueprints/Components/BP_ItemUsableComponent.BP_ItemUsableComponent_C"))
  (bind _returnvalue_4 (`Actor.GetComponentByClass` _returnvalue_2 "/Script/InteractionSystem.InventoryComponent"))
  (`/Engine/EditorBlueprintResources/StandardMacros.IsValid` Interactable
    (:`Is Valid`
      (`/Engine/EditorBlueprintResources/StandardMacros.IsValid` _returnvalue
        (:`Is Valid`
          (`/Engine/EditorBlueprintResources/StandardMacros.IsValid` _returnvalue_2
            (:`Is Valid`
              (`/Engine/EditorBlueprintResources/StandardMacros.IsValid` _returnvalue_3
                (:`Is Valid`
                  (`/Engine/EditorBlueprintResources/StandardMacros.IsValid` _returnvalue_4
                    (:`Is Valid`
                      (for _array_element (`/Game/Blueprints/Components/BP_ItemUsableComponent.GetItemsNeeded` _returnvalue_3)
                        (if (!= (`InventoryComponent.FindItemSlot` _returnvalue_4 _array_element) -1)
                          (`InventoryComponent.RemoveFromInventory` _returnvalue_4 _array_element 1)
                          (`self.OnUseItem` _array_element)
                          (`ItemUsableComponent.OnItemUse` _returnvalue_3 (`self.GetOwner`) _array_element))))))))))))))