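; Actor component that makes its owner a target for item use, tracking which items are still needed to complete it.
; On BeginPlay it binds to its OnItemUse dispatcher; each use of a matching item removes it from ItemsNeeded and plays a use sound at the owner's location.
; When the list empties it fires OnFinishUsable, and GetItemsNeeded exposes the remaining items.
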(event `self.ReceiveBeginPlay`
  (add `self.OnItemUse` (delegate `OnItemUse_Event_0`)))

(event `OnItemUse_Event_0` :!signature `self.OnItemUse`
  (params (User :type "Actor Object Reference") (ItemData :type "ItemData Object Reference"))
  (bind _returnvalue (`KismetArrayLibrary.Array_Find` (`self.ItemsNeeded`) ItemData))
  (if (`KismetArrayLibrary.Array_IsValidIndex` (`self.ItemsNeeded`) _returnvalue)
    (`KismetArrayLibrary.Array_Remove` (`self.ItemsNeeded`) _returnvalue)
    (`GameplayStatics.PlaySoundAtLocation` "/Game/Assets/Licensed/Sound/Cue_UseItem.Cue_UseItem" (`Actor.K2_GetActorLocation` (`self.GetOwner`)) (struct) 1.0 1.0 0.0 null null null)
    (if (`KismetArrayLibrary.Array_IsEmpty` (`self.ItemsNeeded`))
      (`self.OnFinishUsable`))))

(fn `GetItemsNeeded`
  (returns (ItemsNeeded :type "Array of ItemData Object Reference"))
  (return (`self.ItemsNeeded`)))