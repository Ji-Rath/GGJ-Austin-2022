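; BP_Lever is an interactable lever that only works once a lever arm has been attached through its item-usable component.
; Finishing that item use clears the interact prompt, waits briefly, then flags the arm as present and makes it visible.
; Each interaction then flip-flops a timeline that rolls the pivot up to 90 degrees forward or back, finishing the interaction when the timeline completes.
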(event `self.BP_ItemUsableComponent.OnFinishUsable`
  (`InteractableComponent.SetInteractText` (`self.ToggleInteractable`) "")
  (`KismetSystemLibrary.Delay` 0.2) ; Slight delay so interaction doesnt happen immediately
  (set `self.bHasLeverArm` true)
  (`SceneComponent.SetVisibility` (`self.LeverArm`) true false))

(event `self.ToggleInteractable.OnInteract`
  (params (Interactor :type "Actor Object Reference"))
  (if (`self.bHasLeverArm`)
    (`/Engine/EditorBlueprintResources/StandardMacros.FlipFlop`
      (:`A`
        (bind (_direction _newtrack_0) (`Timeline|LeverToggle` :!label _label)
          (:`Update`
            (`SceneComponent.K2_SetRelativeRotation` (`self.LeverPivot`) (`KismetMathLibrary.MakeRotator` (* _newtrack_0 90.0)) false false))
          (:`Finished`
            (`InteractableComponent.FinishInteraction` (`self.ToggleInteractable`) true))))
      (:`B`
        (goto _label :!via `Reverse`)))))

(fn `UserConstructionScript`)